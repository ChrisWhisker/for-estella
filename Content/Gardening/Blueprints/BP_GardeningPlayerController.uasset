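; Player controller for the gardening game that manages the HUD, pause menu and music ducking.
; On BeginPlay it creates and shows the HUD, then caches the first AmbientSound actor as the music source along with its original volume.
; The Pause input lazily creates the pause widget, switches to UI-only input, removes the HUD, halves the music volume if audible and pauses the game.
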(event `self.ReceiveBeginPlay`
  (`parent.ReceiveBeginPlay`)
  (`self.AddHud`)
  (bind _returnvalue (`GameplayStatics.GetActorOfClass` "/Script/Engine.AmbientSound"))
  (bind _output_get (set `self.MusicActor` _returnvalue))
  (set `self.MusicOriginalVolume` (`AudioComponent.VolumeMultiplier` (`AmbientSound.AudioComponent` _output_get))))

(event `InputAction|Pause`
  (params (Key :type "Key Structure"))
  (bind _pausemenureference (`self.PauseMenuReference`))
  (bind _audiocomponent (`AmbientSound.AudioComponent` (`self.MusicActor`)))
  (:`Pressed`
    (`/Engine/EditorBlueprintResources/StandardMacros.IsValid` (`self.PauseMenuReference`)
      (:`Is Valid`
        _)
      (:`Is Not Valid`
        (bind _returnvalue (`|CreateWidget` "/Game/Gardening/UI/WBP_PauseMenu.WBP_PauseMenu_C"))
        (set `self.PauseMenuReference` _returnvalue)))
    (set `self.bShowMouseCursor` true)
    (`WidgetBlueprintLibrary.SetInputMode_UIOnlyEx` self _pausemenureference)
    (`UserWidget.AddToViewport` _pausemenureference 0)
    (`Widget.RemoveFromParent` (`self.HudReference`))
    (if (> (`AudioComponent.VolumeMultiplier` _audiocomponent) 0.0)
      (`AudioComponent.SetVolumeMultiplier` _audiocomponent (/ (`self.MusicOriginalVolume`) 2.0)))
    (`GameplayStatics.SetGamePaused` true)))

(fn `AddHud`
  (`/Engine/EditorBlueprintResources/StandardMacros.IsValid` (`self.HudReference`)
    (:`Is Valid`
      _)
    (:`Is Not Valid`
      (bind _returnvalue (`|CreateWidget` (`self.HudClass_0`)))
      (bind _output_get (set `self.HudReference` _returnvalue))))
  (`UserWidget.AddToViewport` _output_get 0))

(fn `UserConstructionScript`)