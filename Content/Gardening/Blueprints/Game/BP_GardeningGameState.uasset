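; Game state for a gardening game that tracks plants and garden height for two sides, player and AI.
; Events add or remove plants in separate per-team arrays, with team 0 as the player and any other number as the AI.
; AddGardenHeight adds feet to the chosen team's total, clamps it at zero or above, and prints a debug message for AI changes.
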(event `self.ReceiveTick`
  (params (DeltaSeconds :type "Float (single-precision)")))

(event `self.AddGardenHeightFeet`
  (params (TeamNumber :type Integer) (FeetToAdd :type "Float (single-precision)"))
  (`self.AddGardenHeight` TeamNumber FeetToAdd))

(event `self.AddPlantToGarden`
  (params (TeamNumber :type Integer) (Plant :type "Plant Object Reference"))
  (if (== TeamNumber 0)
    (`KismetArrayLibrary.Array_AddUnique` (`self.PlayerPlants`) Plant)
    (else
      (`KismetArrayLibrary.Array_AddUnique` (`self.AIPlants`) Plant))))

(event `self.RemovePlantFromGarden`
  (params (TeamNumber :type Integer) (Plant :type "Plant Object Reference"))
  (if (== TeamNumber 0)
    (`KismetArrayLibrary.Array_RemoveItem` (`self.PlayerPlants`) Plant)
    (else
      (`KismetArrayLibrary.Array_RemoveItem` (`self.AIPlants`) Plant))))

(fn `AddGardenHeight`
  (params (TeamNumber :type Integer) (FeetToAdd :type "Float (double-precision)"))
  (locals (TeamGardenHeight :type "Float (double-precision)"))
  (bind _output_get (set `local.TeamGardenHeight` (`KismetMathLibrary.SelectFloat` (`self.PlayerGardenHeightFeet`) (`self.AIGardenHeightFeet`) (== TeamNumber 0))))
  (if (== (`local.TeamNumber`) 0)
    (bind _returnvalue (`KismetMathLibrary.FClamp` (+ _output_get (`local.FeetToAdd`)) 0.0 7.766279436516721e+18))
    (bind _output_get_2 (set `self.PlayerGardenHeightFeet` _returnvalue))
    (else
      (set `self.AIGardenHeightFeet` _returnvalue)
      (`KismetSystemLibrary.PrintString` (`KismetStringLibrary.Concat_StrStr` "Added " (`KismetStringLibrary.Conv_DoubleToString` 0.0) " to AI garden height")))))

(fn `UserConstructionScript`)